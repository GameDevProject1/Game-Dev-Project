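; Base actor for platformer collectables: keys and shrink or grow potions that Alice picks up with the collect input.
; Sphere overlap with Normal_Alice enables the actor's input, and leaving disables it.
; Collecting requires Normal_GameMode, destroys the actor, then switches on CollectableType.
; Potions set the matching Has flag on Alice and show a message widget, while keys only print a string.
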(event `EnhancedInput|/Game/ThirdPerson/Input/Actions/IA_Collect`
  (params (ActionValue :type Boolean) (ElapsedSeconds :type "Float (double-precision)") (TriggeredSeconds :type "Float (double-precision)") (InputAction :type "InputAction Object Reference" :default "/Game/ThirdPerson/Input/Actions/IA_Collect.IA_Collect"))
  (bind _returnvalue (`GameplayStatics.GetPlayerPawn` 0))
  (:`Started`
    (cast `/Game/ThirdPerson/Blueprints/Normal_GameMode` (`GameplayStatics.GetGameMode`))
    (`self.K2_DestroyActor`)
    (switch `/Game/Custom/Assets/PlatformerCollectables/ECollectableType` (`self.CollectableType`)
      (:`NewEnumerator0`
        (`KismetSystemLibrary.PrintString` "Key Collected!"))
      (:`NewEnumerator1`
        (`KismetSystemLibrary.PrintString` "Shrink Potion Collected!")
        (bind _asnormal_alice (cast `/Game/ThirdPerson/Blueprints/Normal_Alice` _returnvalue))
        (set `/Game/ThirdPerson/Blueprints/Normal_Alice.HasPotionShrink` true _asnormal_alice)
        (bind _returnvalue_2 (`|CreateWidget` "/Game/Custom/Assets/PlatformerCollectables/WBP_PotionMessage.WBP_PotionMessage_C" :!label _label))
        (`UserWidget.AddToViewport` _returnvalue_2 0))
      (:`NewEnumerator2`
        (`KismetSystemLibrary.PrintString` "Grow Potion Collected!")
        (bind _asnormal_alice_2 (cast `/Game/ThirdPerson/Blueprints/Normal_Alice` _returnvalue))
        (set `/Game/ThirdPerson/Blueprints/Normal_Alice.HasPotionGrow` true _asnormal_alice_2)
        (goto _label)))))

(event `self.Sphere.OnComponentBeginOverlap`
  (params (OverlappedComponent :type "PrimitiveComponent Object Reference") (OtherActor :type "Actor Object Reference") (OtherComp :type "PrimitiveComponent Object Reference") (OtherBodyIndex :type Integer) (bFromSweep :type Boolean) (SweepResult :type "HitResult Structure (by ref)"))
  (cast `/Game/ThirdPerson/Blueprints/Normal_Alice` OtherActor)
  (`self.EnableInput` (`GameplayStatics.GetPlayerController` 0)))

(event `self.Sphere.OnComponentEndOverlap`
  (params (OverlappedComponent :type "PrimitiveComponent Object Reference") (OtherActor :type "Actor Object Reference") (OtherComp :type "PrimitiveComponent Object Reference") (OtherBodyIndex :type Integer))
  (cast `/Game/ThirdPerson/Blueprints/Normal_Alice` OtherActor)
  (`self.DisableInput` (`GameplayStatics.GetPlayerController` 0)))

(fn `UserConstructionScript`)