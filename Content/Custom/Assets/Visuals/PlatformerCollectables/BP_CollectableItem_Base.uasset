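; Base collectable actor for keys and shrink or grow potions that Normal_Alice picks up with the IA_Collect input.
; After a short BeginPlay delay it caches the player and the HUD from Normal_GameMode.
; Sphere overlap toggles its input and the player's collection-area flag, refreshing guide text.
; Collecting destroys the actor, then switches on CollectableType to update player inventory and HUD.
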(event `EnhancedInput|/Game/ThirdPerson/Input/Actions/IA_Collect`
  (params (ActionValue :type Boolean) (ElapsedSeconds :type "Float (double-precision)") (TriggeredSeconds :type "Float (double-precision)") (InputAction :type "InputAction Object Reference" :default "/Game/ThirdPerson/Input/Actions/IA_Collect.IA_Collect"))
  (bind _playerref (`self.PlayerRef`))
  (bind _hudref (`self.HudRef`))
  (:`Started`
    (cast `/Game/ThirdPerson/Blueprints/Normal_GameMode` (`GameplayStatics.GetGameMode`))
    (`self.K2_DestroyActor`)
    (switch `/Game/Custom/Assets/Visuals/PlatformerCollectables/ECollectableType` (`self.CollectableType`)
      (:`NewEnumerator0`
        (`KismetSystemLibrary.PrintString` "Key Collected!")
        (set `/Game/ThirdPerson/Blueprints/Normal_Alice.KeyCount` (+ (`/Game/ThirdPerson/Blueprints/Normal_Alice.KeyCount` _playerref) 1) _playerref)
        (`/Game/Custom/Assets/Visuals/PlatformerCollectables/WB_HUD.UpdateKeys` _hudref))
      (:`NewEnumerator1`
        (`KismetSystemLibrary.PrintString` "Shrink Potion Collected!")
        (set `/Game/ThirdPerson/Blueprints/Normal_Alice.HasPotionShrink` true _playerref)
        (`/Game/Custom/Assets/Visuals/PlatformerCollectables/WB_HUD.UpdateGuideText` _hudref :!label _label))
      (:`NewEnumerator2`
        (`KismetSystemLibrary.PrintString` "Grow Potion Collected!")
        (set `/Game/ThirdPerson/Blueprints/Normal_Alice.HasPotionGrow` true _playerref)
        (goto _label)))))

(event `self.ReceiveBeginPlay`
  (`KismetSystemLibrary.Delay` 0.2)
  (bind _asnormal_alice (cast `/Game/ThirdPerson/Blueprints/Normal_Alice` (`GameplayStatics.GetPlayerPawn` 0)))
  (set `self.PlayerRef` _asnormal_alice)
  (bind _asnormal_game_mode (cast `/Game/ThirdPerson/Blueprints/Normal_GameMode` (`GameplayStatics.GetGameMode`)))
  (bind _output_get (set `self.HudRef` (`/Game/ThirdPerson/Blueprints/Normal_GameMode.HUD` _asnormal_game_mode)))
  (`KismetSystemLibrary.PrintText` (`KismetTextLibrary.Conv_ObjectToText` _output_get)))

(event `self.Sphere.OnComponentBeginOverlap`
  (params (OverlappedComponent :type "PrimitiveComponent Object Reference") (OtherActor :type "Actor Object Reference") (OtherComp :type "PrimitiveComponent Object Reference") (OtherBodyIndex :type Integer) (bFromSweep :type Boolean) (SweepResult :type "HitResult Structure (by ref)"))
  (cast `/Game/ThirdPerson/Blueprints/Normal_Alice` OtherActor)
  (`self.EnableInput` (`GameplayStatics.GetPlayerController` 0))
  (set `/Game/ThirdPerson/Blueprints/Normal_Alice.IsCollectionArea` true (`self.PlayerRef`))
  (`/Game/Custom/Assets/Visuals/PlatformerCollectables/WB_HUD.UpdateGuideText` (`self.HudRef`) :!label _label_2))

(event `self.Sphere.OnComponentEndOverlap`
  (params (OverlappedComponent :type "PrimitiveComponent Object Reference") (OtherActor :type "Actor Object Reference") (OtherComp :type "PrimitiveComponent Object Reference") (OtherBodyIndex :type Integer))
  (cast `/Game/ThirdPerson/Blueprints/Normal_Alice` OtherActor)
  (`self.DisableInput` (`GameplayStatics.GetPlayerController` 0))
  (set `/Game/ThirdPerson/Blueprints/Normal_Alice.IsCollectionArea` false (`self.PlayerRef`))
  (goto _label_2))

(fn `UserConstructionScript`)