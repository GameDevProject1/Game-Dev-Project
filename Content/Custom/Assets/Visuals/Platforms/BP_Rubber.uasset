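; BP_Rubber is a bouncy rubber platform that launches the Normal_Alice character back up when she hits it.
; A hit on the platform component negates her last-update vertical velocity, scales it by Bounciness and applies it through LaunchCharacter if it exceeds MinBounceHeight.
; Weaker impacts instead set her NormalJumpVelocity to a multiplied jump velocity, which this Blueprint never resets.
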(event `self.ReceiveBeginPlay`
  ;[1 1 1] Set platform variable
  (bind _output_get (set `self.Platform` (`self.RubberPlatform`)))
  (add `PrimitiveComponent.OnComponentHit` _output_get (delegate `On Platform Hit`)))

(event `On Platform Hit`
  (params (HitComponent :type "PrimitiveComponent Object Reference") (OtherActor :type "Actor Object Reference") (OtherComp :type "PrimitiveComponent Object Reference") (NormalImpulse :type "Vector Structure") (Hit :type "HitResult Structure (by ref)"))
  (bind (_returnvalue_x _returnvalue_y _returnvalue_z) (`KismetMathLibrary.BreakVector` (`CharacterMovementComponent.GetLastUpdateVelocity` (`Character.CharacterMovement` (`self.Alice`)))))
  (bind _asnormal_alice (cast `/Game/ThirdPerson/Blueprints/Normal_Alice` OtherActor))
  (set `self.Alice` _asnormal_alice)
  (set `self.BounceHeight` (* (* _returnvalue_z -1.0) (`self.Bounciness`)))
  ;[1 1 1] Launch as long as it's higher than MinBounceHeight
  (if (> (`self.BounceHeight`) (`self.MinBounceHeight`))
    (`Character.LaunchCharacter` (`self.Alice`) (`KismetMathLibrary.MakeVector` 0.0 0.0 (`self.BounceHeight`)) false true)
    (else
      ;[1 1 1] Jump height when standing on the platform
      (set `/Game/ThirdPerson/Blueprints/Normal_Alice.NormalJumpVelocity` (* (`self.JumpVelocity`) (`self.JumpMultiplier`)) (`self.Alice`)))))

(fn `UserConstructionScript`)