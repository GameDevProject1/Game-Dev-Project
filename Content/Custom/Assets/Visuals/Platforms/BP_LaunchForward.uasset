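; Launch pad platform Blueprint that throws the player character forward and upward when touched.
; On BeginPlay it binds a hit event to its platform mesh component.
; When Normal_Alice hits it, it plays a boing sound and launches her along the platform's horizontal forward vector, with configurable forward and vertical speeds.
; The launch always overrides vertical velocity, while horizontal override is configurable.
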(event `self.ReceiveBeginPlay`
  ;[1 1 1] Set platform variable
  (bind _output_get (set `self.Platform` (`self.PlatformBlack`)))
  (add `PrimitiveComponent.OnComponentHit` _output_get (delegate `On Platform Hit`)))

(event `On Platform Hit`
  (params (HitComponent :type "PrimitiveComponent Object Reference") (OtherActor :type "Actor Object Reference") (OtherComp :type "PrimitiveComponent Object Reference") (NormalImpulse :type "Vector Structure") (Hit :type "HitResult Structure (by ref)"))
  (bind _launchforwardvelocity (`self.LaunchForwardVelocity`))
  (bind (_returnvalue_x _returnvalue_y) (`KismetMathLibrary.BreakVector` (`KismetMathLibrary.GetForwardVector` (`SceneComponent.K2_GetComponentRotation` (`self.Platform`)))))
  (bind _asnormal_alice (cast `/Game/ThirdPerson/Blueprints/Normal_Alice` OtherActor))
  ;[1 1 1] Play sound
  (`GameplayStatics.PlaySoundAtLocation` "/Game/Custom/Assets/Audio/platforms/boing.boing" (`self.K2_GetActorLocation` _asnormal_alice) (struct) 1.0 1.0 0.0 null null null null)
  ;[1 1 1] launch
  (`Character.LaunchCharacter` _asnormal_alice (`KismetMathLibrary.MakeVector` (* _returnvalue_x _launchforwardvelocity) (* _returnvalue_y _launchforwardvelocity) (`self.LaunchVelocityZ`)) (`self.XYOverride`) true))

(fn `UserConstructionScript`)