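; BP_DoubleJump is a bounce platform that launches the Normal_Alice character upward and changes her jump abilities.
; BeginPlay binds the DoubleJumpPlatform component's hit event, which filters for Normal_Alice, plays a Boing sound and launches her with Z velocity override.
; The hit also sets her max jump count and, unless UseCharacterJumpVelocity is set, her jump Z velocity.
; Nothing in this Blueprint restores those jump values afterward.
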(event `self.ReceiveBeginPlay`
  ;[1 1 1] Set platform variable
  (bind _output_get (set `self.Platform` (`self.DoubleJumpPlatform`)))
  (add `PrimitiveComponent.OnComponentHit` _output_get (delegate `On Platform Hit`)))

(event `On Platform Hit`
  (params (HitComponent :type "PrimitiveComponent Object Reference") (OtherActor :type "Actor Object Reference") (OtherComp :type "PrimitiveComponent Object Reference") (NormalImpulse :type "Vector Structure") (Hit :type "HitResult Structure (by ref)"))
  ;[1 1 1] Launch
  (bind _asnormal_alice (cast `/Game/ThirdPerson/Blueprints/Normal_Alice` OtherActor))
  ;;[1 1 1] Play sound
  (`GameplayStatics.PlaySoundAtLocation` "/Game/Custom/Assets/Audio/platforms/boing.boing" (`self.K2_GetActorLocation` _asnormal_alice) (struct) 1.0 1.0 0.0 null null null null)
  (`Character.LaunchCharacter` _asnormal_alice (`KismetMathLibrary.MakeVector` 0.0 0.0 (`self.LaunchVelocity`)) false true)
  ;[1 1 1] Set jump count and height
  (set `Character.JumpMaxCount` (`self.JumpCount`) _asnormal_alice)
  (if (not (`self.UseCharacterJumpVelocity`))
    (set `CharacterMovementComponent.JumpZVelocity` (`self.JumpVelocity`) (`Character.CharacterMovement` _asnormal_alice))))

(fn `UserConstructionScript`)