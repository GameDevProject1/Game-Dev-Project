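; Trampoline platform that bounces via physics simulation, reacting to the player character landing on it.
; On BeginPlay it constrains the platform mesh to a physics constraint, enables simulation, and applies configurable mass, damping and linear drive spring strength.
; When hit by Normal_Alice with TransferVelocity enabled, it copies the character's vertical movement velocity onto the platform so the landing impact compresses the spring.
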(event `self.ReceiveBeginPlay`
  (bind _platform (`self.Platform`))
  (bind _platform_2 (`self.Platform`))
  ;[1 1 1] Set platform variable
  (set `self.Platform` (`self.TrampolinePlatform`))
  (`PhysicsConstraintComponent.SetConstrainedComponents` (`self.PhysicsConstraint`) _platform "None" null "None")
  (`PrimitiveComponent.SetSimulatePhysics` _platform true)
  ;[1 1 1] Set default variables
  (`PrimitiveComponent.SetMassOverrideInKg` _platform_2 "None" (`self.Mass`) true)
  (`PrimitiveComponent.SetLinearDamping` _platform_2 (`self.Damping`))
  (`PhysicsConstraintComponent.SetLinearDriveParams` (`self.PhysicsConstraint`) (`self.Strength`) 0.0 0.0)
  (add `PrimitiveComponent.OnComponentHit` (`self.Platform`) (delegate `On Platform Hit`)))

(event `On Platform Hit`
  (params (HitComponent :type "PrimitiveComponent Object Reference") (OtherActor :type "Actor Object Reference") (OtherComp :type "PrimitiveComponent Object Reference") (NormalImpulse :type "Vector Structure") (Hit :type "HitResult Structure (by ref)"))
  ;[1 1 1] Transfer velocity to platform
  (if (`self.TransferVelocity`)
    (bind _asnormal_alice (cast `/Game/ThirdPerson/Blueprints/Normal_Alice` OtherActor))
    (bind (_returnvalue_x _returnvalue_y _returnvalue_z) (`KismetMathLibrary.BreakVector` (`CharacterMovementComponent.GetLastUpdateVelocity` (`Character.CharacterMovement` _asnormal_alice))))
    (`PrimitiveComponent.SetPhysicsLinearVelocity` HitComponent (`KismetMathLibrary.MakeVector` 0.0 0.0 _returnvalue_z) false "None")))

(fn `UserConstructionScript`)