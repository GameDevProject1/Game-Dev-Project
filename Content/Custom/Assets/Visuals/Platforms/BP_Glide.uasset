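; BP_Glide is a platform that bounces Alice upward and primes her for a single glide.
; On begin play it binds to the hit event of its black platform component and responds only to Normal_Alice.
; A hit plays a boing sound, stops any active glide to prevent a zero-gravity jump, then launches her.
; It then enables apex notification and passes its glide gravity, velocity and air control to the character.
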(event `self.ReceiveBeginPlay`
  ;[1 1 1] Set platform variable
  (bind _output_get (set `self.Platform` (`self.PlatformBlack`)))
  (add `PrimitiveComponent.OnComponentHit` _output_get (delegate `On Platform Hit`)))

(event `On Platform Hit`
  (params (HitComponent :type "PrimitiveComponent Object Reference") (OtherActor :type "Actor Object Reference") (OtherComp :type "PrimitiveComponent Object Reference") (NormalImpulse :type "Vector Structure") (Hit :type "HitResult Structure (by ref)"))
  (bind _alice (`self.Alice`))
  (bind _alice_2 (`self.Alice`))
  ;[1 1 1] Launch
  (bind _asnormal_alice (cast `/Game/ThirdPerson/Blueprints/Normal_Alice` OtherActor))
  (bind _output_get (set `self.Alice` _asnormal_alice))
  ;;[1 1 1] Play sound
  (`GameplayStatics.PlaySoundAtLocation` "/Game/Custom/Assets/Audio/platforms/boing.boing" (`self.K2_GetActorLocation` _output_get) (struct) 1.0 1.0 0.0 null null null null)
  ;;[1 1 1] Prevent zero gravity jump
  (`/Game/ThirdPerson/Blueprints/Normal_Alice.StopGliding` _alice)
  (`Character.LaunchCharacter` _alice (`KismetMathLibrary.MakeVector` 0.0 0.0 (`self.LaunchVelocity`)) false false)
  ;[1 1 1] Set character variables for gliding
  (set `/Game/ThirdPerson/Blueprints/Normal_Alice.willGlideOnce` true _alice_2)
  (set `CharacterMovementComponent.bNotifyApex` true (`Character.CharacterMovement` _alice_2))
  (set `/Game/ThirdPerson/Blueprints/Normal_Alice.GlideGravity` (`self.GlideGravity`) _alice_2)
  (set `/Game/ThirdPerson/Blueprints/Normal_Alice.GlideVelocity` (`self.GlideVelocity`) _alice_2)
  (set `/Game/ThirdPerson/Blueprints/Normal_Alice.GlideAirControl` (`self.GlideAirControl`) _alice_2))

(fn `UserConstructionScript`)