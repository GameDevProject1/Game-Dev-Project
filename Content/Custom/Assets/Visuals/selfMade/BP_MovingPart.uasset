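; BP_MovingPart is an actor that eases a MovingPart component back and forth between the relative locations of A and B.
; MoveWall alternates direction via MoveTo, optionally starting at BeginPlay and, with PingPong, repeating after a pause.
; When MoveWhenCharacterIsNear is false, an overlap in NoMoveZone blocks new moves.
; Ending any overlap clears CharacterIsNear and calls MoveWall again.
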(event `self.ReceiveBeginPlay`
  ;[1 1 1] Check if movement is started with the game
  (if (`self.startAtPlay`)
    (`self.MoveWall`)))

(event `MoveWall`
  (bind _translationtime (`self.translationTime`))
  (bind _movingpart (`self.movingPart`))
  ;[1 1 1] check if the character has influence and is there
  (if (`self.Move when Character is Near`)
    ;[1 1 1] Decide direction
    (if (`self.moveTo`) :!label _label
      ;[1 1 1] actually move the component
      (`KismetSystemLibrary.MoveComponentTo` _movingpart (`SceneComponent.RelativeLocation` (`self.A`)) (struct) true true _translationtime)
      ;[1 1 1] Reset variables and chek for endless moving
      (set `self.moveTo` false)
      (else
        (`KismetSystemLibrary.MoveComponentTo` _movingpart (`SceneComponent.RelativeLocation` (`self.B`)) (struct) true true _translationtime)
        (set `self.moveTo` true)))
    (if (`self.pingPong`)
      (`KismetSystemLibrary.Delay` (`self.pinpPongPause`))
      (`self.MoveWall`))
    (elif (not (`self.Character is near`))
      (goto _label))))

(event `self.noMoveZone.OnComponentBeginOverlap`
  (params (OverlappedComponent :type "PrimitiveComponent Object Reference") (OtherActor :type "Actor Object Reference") (OtherComp :type "PrimitiveComponent Object Reference") (OtherBodyIndex :type Integer) (bFromSweep :type Boolean) (SweepResult :type "HitResult Structure (by ref)"))
  ;[1 1 1] Check if Character is in reach
  (set `self.Character is near` true))

(event `self.noMoveZone.OnComponentEndOverlap`
  (params (OverlappedComponent :type "PrimitiveComponent Object Reference") (OtherActor :type "Actor Object Reference") (OtherComp :type "PrimitiveComponent Object Reference") (OtherBodyIndex :type Integer))
  ;[1 1 1] Check if Character is in reach
  (set `self.Character is near` false)
  (`self.MoveWall`))

(fn `UserConstructionScript`)