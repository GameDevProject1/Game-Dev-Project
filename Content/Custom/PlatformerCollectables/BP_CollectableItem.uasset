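; BP_CollectableItem is a platformer pickup that the player collects by pressing the collect input while near it.
; Its Sphere overlap with Normal_Alice enables input on the actor, and leaving the sphere disables it.
; On IA_Collect it decrements Remaining on Normal_GameMode, adds a WB_Collected widget to the viewport, then destroys itself.
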(event `EnhancedInput|/Game/ThirdPerson/Input/Actions/IA_Collect`
  (params (ActionValue :type Boolean) (ElapsedSeconds :type "Float (double-precision)") (TriggeredSeconds :type "Float (double-precision)") (InputAction :type "InputAction Object Reference" :default "/Game/ThirdPerson/Input/Actions/IA_Collect.IA_Collect"))
  (:`Started`
    (bind _asnormal_game_mode (cast `/Game/ThirdPerson/Blueprints/Normal_GameMode` (`GameplayStatics.GetGameMode`)))
    (bind _result (`/Engine/EditorBlueprintResources/StandardMacros.DecrementInt` (`/Game/ThirdPerson/Blueprints/Normal_GameMode.Remaining` _asnormal_game_mode))
      (:`  `
        (set `/Game/ThirdPerson/Blueprints/Normal_GameMode.Remaining` _result _asnormal_game_mode)
        (bind _returnvalue (`|CreateWidget` "/Game/Custom/PlatformerCollectables/WB_Collected.WB_Collected_C"))
        (`UserWidget.AddToViewport` _returnvalue 0)
        (`self.K2_DestroyActor`)))))

(event `self.Sphere.OnComponentBeginOverlap`
  (params (OverlappedComponent :type "PrimitiveComponent Object Reference") (OtherActor :type "Actor Object Reference") (OtherComp :type "PrimitiveComponent Object Reference") (OtherBodyIndex :type Integer) (bFromSweep :type Boolean) (SweepResult :type "HitResult Structure (by ref)"))
  (cast `/Game/ThirdPerson/Blueprints/Normal_Alice` OtherActor)
  (`self.EnableInput` (`GameplayStatics.GetPlayerController` 0)))

(event `self.Sphere.OnComponentEndOverlap`
  (params (OverlappedComponent :type "PrimitiveComponent Object Reference") (OtherActor :type "Actor Object Reference") (OtherComp :type "PrimitiveComponent Object Reference") (OtherBodyIndex :type Integer))
  (cast `/Game/ThirdPerson/Blueprints/Normal_Alice` OtherActor)
  (`self.DisableInput` (`GameplayStatics.GetPlayerController` 0)))

(fn `UserConstructionScript`)