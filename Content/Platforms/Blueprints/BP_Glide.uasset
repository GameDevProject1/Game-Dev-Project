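; BP_Glide is a bounce platform that launches Normal_Alice upward and primes her for a one-time glide.
; On Box overlap it plays the Boing sound at the overlapping actor, cancels any active glide to prevent a zero-gravity jump, then launches the character.
; It enables apex notification and copies its glide gravity, velocity and air control to the character, which holds the glide logic.
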(event `self.Box.OnComponentBeginOverlap`
  (params (OverlappedComponent :type "PrimitiveComponent Object Reference") (OtherActor :type "Actor Object Reference") (OtherComp :type "PrimitiveComponent Object Reference") (OtherBodyIndex :type Integer) (bFromSweep :type Boolean) (SweepResult :type "HitResult Structure (by ref)"))
  ;[1 1 1] Turn on gliding
  (`GameplayStatics.PlaySoundAtLocation` "/Game/Custom/Assets/Audio/platforms/boing.boing" (`self.K2_GetActorLocation` OtherActor) (struct) 1.0 1.0 0.0 null null null null)
  (bind _asnormal_alice (cast `/Game/ThirdPerson/Blueprints/Normal_Alice` OtherActor))
  ;[1 1 1] Prevent zero gravity jump
  (`/Game/ThirdPerson/Blueprints/Normal_Alice.StopGliding` _asnormal_alice)
  (`Character.LaunchCharacter` _asnormal_alice (`KismetMathLibrary.MakeVector` 0.0 0.0 (`self.LaunchVelocity`)) false false)
  (set `/Game/ThirdPerson/Blueprints/Normal_Alice.willGlideOnce` true _asnormal_alice)
  (set `CharacterMovementComponent.bNotifyApex` true (`Character.CharacterMovement` _asnormal_alice))
  ;[1 1 1] Set character variables for gliding
  (set `/Game/ThirdPerson/Blueprints/Normal_Alice.GlideGravity` (`self.GlideGravity`) _asnormal_alice)
  (set `/Game/ThirdPerson/Blueprints/Normal_Alice.GlideVelocity` (`self.GlideVelocity`) _asnormal_alice)
  (set `/Game/ThirdPerson/Blueprints/Normal_Alice.GlideAirControl` (`self.GlideAirControl`) _asnormal_alice))

(fn `UserConstructionScript`)