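; BP_DoubleJump is a launch platform that bounces the Normal_Alice character upward and changes her jump ability.
; On Box overlap it plays a Boing sound at any entering actor, then casts to Normal_Alice and launches her with Z override.
; It then sets her max jump count and, unless UseCharacterJumpVelocity is set, her jump Z velocity.
; Nothing in this Blueprint restores those jump values afterwards.
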(event `self.Box.OnComponentBeginOverlap`
  (params (OverlappedComponent :type "PrimitiveComponent Object Reference") (OtherActor :type "Actor Object Reference") (OtherComp :type "PrimitiveComponent Object Reference") (OtherBodyIndex :type Integer) (bFromSweep :type Boolean) (SweepResult :type "HitResult Structure (by ref)"))
  ;[1 1 1] launch
  (`GameplayStatics.PlaySoundAtLocation` "/Game/Custom/Assets/Audio/platforms/boing.boing" (`self.K2_GetActorLocation` OtherActor) (struct) 1.0 1.0 0.0 null null null null)
  (bind _asnormal_alice (cast `/Game/ThirdPerson/Blueprints/Normal_Alice` OtherActor))
  (`Character.LaunchCharacter` _asnormal_alice (`KismetMathLibrary.MakeVector` 0.0 0.0 (`self.LaunchVelocity`)) false true)
  (set `Character.JumpMaxCount` (`self.JumpCount`) _asnormal_alice)
  (if (not (`self.UseCharacterJumpVelocity`))
    (set `CharacterMovementComponent.JumpZVelocity` (`self.JumpVelocity`) (`Character.CharacterMovement` _asnormal_alice))))

(fn `UserConstructionScript`)