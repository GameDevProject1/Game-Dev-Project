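; BP_Rubber is a bouncy platform that reacts when Normal_Alice hits its GlidePlatform component.
; On hit, it sets her jump Z velocity to JumpVelocity scaled by JumpMultiplier, with no reset in this Blueprint.
; It also inverts her last vertical velocity, scales it by Bounciness, and launches her upward with Z override when the result exceeds MinBounceHeight.
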(event `self.GlidePlatform.OnComponentHit`
  (params (HitComponent :type "PrimitiveComponent Object Reference") (OtherActor :type "Actor Object Reference") (OtherComp :type "PrimitiveComponent Object Reference") (NormalImpulse :type "Vector Structure") (Hit :type "HitResult Structure (by ref)"))
  (bind _asnormal_alice (cast `/Game/ThirdPerson/Blueprints/Normal_Alice` OtherActor))
  (bind _charactermovement (`Character.CharacterMovement` _asnormal_alice))
  (set `CharacterMovementComponent.JumpZVelocity` (* (`self.JumpVelocity`) (`self.JumpMultiplier`)) _charactermovement)
  (bind (_returnvalue_x _returnvalue_y _returnvalue_z) (`KismetMathLibrary.BreakVector` (`CharacterMovementComponent.GetLastUpdateVelocity` _charactermovement)))
  (bind _returnvalue (* (* _returnvalue_z -1.0) (`self.Bounciness`)))
  (if (> _returnvalue (`self.MinBounceHeight`))
    (`Character.LaunchCharacter` _asnormal_alice (`KismetMathLibrary.MakeVector` 0.0 0.0 _returnvalue) false true)))

(fn `UserConstructionScript`)