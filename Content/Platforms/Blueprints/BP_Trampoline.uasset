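; Trampoline platform Blueprint built on a physics-simulated platform with a spring-like constraint drive, tuned on BeginPlay through mass, damping and strength variables.
; When Normal_Alice hits the platform, her last vertical movement velocity becomes the platform's linear Z velocity.
; A Box trigger switches her capsule to QueryAndProbe collision while overlapping to allow bounciness, then restores QueryAndPhysics on exit.
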(event `self.ReceiveBeginPlay`
  (bind _trampolineplatform (`self.TrampolinePlatform`))
  ;[1 1 1] Set default variables
  (`PrimitiveComponent.SetMassOverrideInKg` _trampolineplatform "None" (`self.Mass`) true)
  (`PrimitiveComponent.SetLinearDamping` _trampolineplatform (`self.Damping`))
  (`PhysicsConstraintComponent.SetLinearDriveParams` (`self.PhysicsConstraint`) (`self.Strength`) 0.0 0.0))

(event `self.TrampolinePlatform.OnComponentHit`
  (params (HitComponent :type "PrimitiveComponent Object Reference") (OtherActor :type "Actor Object Reference") (OtherComp :type "PrimitiveComponent Object Reference") (NormalImpulse :type "Vector Structure") (Hit :type "HitResult Structure (by ref)"))
  ;[1 1 1] Transfer velocity to platform
  (bind _asnormal_alice (cast `/Game/ThirdPerson/Blueprints/Normal_Alice` OtherActor))
  (bind (_returnvalue_x _returnvalue_y _returnvalue_z) (`KismetMathLibrary.BreakVector` (`CharacterMovementComponent.GetLastUpdateVelocity` (`Character.CharacterMovement` _asnormal_alice))))
  (`PrimitiveComponent.SetPhysicsLinearVelocity` (`self.TrampolinePlatform`) (`KismetMathLibrary.MakeVector` 0.0 0.0 _returnvalue_z) false "None"))

(event `self.Box.OnComponentBeginOverlap`
  (params (OverlappedComponent :type "PrimitiveComponent Object Reference") (OtherActor :type "Actor Object Reference") (OtherComp :type "PrimitiveComponent Object Reference") (OtherBodyIndex :type Integer) (bFromSweep :type Boolean) (SweepResult :type "HitResult Structure (by ref)"))
  ;[1 1 1] Set collision type to allow bounciness
  (bind _asnormal_alice (cast `/Game/ThirdPerson/Blueprints/Normal_Alice` OtherActor))
  (`PrimitiveComponent.SetCollisionEnabled` (`Character.CapsuleComponent` _asnormal_alice) "QueryAndProbe"))

(event `self.Box.OnComponentEndOverlap`
  (params (OverlappedComponent :type "PrimitiveComponent Object Reference") (OtherActor :type "Actor Object Reference") (OtherComp :type "PrimitiveComponent Object Reference") (OtherBodyIndex :type Integer))
  ;[1 1 1] Set collision type to allow bounciness
  (bind _asnormal_alice (cast `/Game/ThirdPerson/Blueprints/Normal_Alice` OtherActor))
  (`PrimitiveComponent.SetCollisionEnabled` (`Character.CapsuleComponent` _asnormal_alice) "QueryAndPhysics"))

(fn `UserConstructionScript`)