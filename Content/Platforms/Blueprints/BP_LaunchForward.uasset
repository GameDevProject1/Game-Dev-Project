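; BP_LaunchForward is a launch platform that throws the Normal_Alice player character forward and upward when it touches the box.
; Box overlap plays the Boing sound at any overlapping actor, then launches only a successful Normal_Alice cast.
; Horizontal velocity follows the GlidePlatform's world forward vector scaled by a forward speed, while vertical velocity always overrides and horizontal override is configurable.
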(event `self.Box.OnComponentBeginOverlap`
  (params (OverlappedComponent :type "PrimitiveComponent Object Reference") (OtherActor :type "Actor Object Reference") (OtherComp :type "PrimitiveComponent Object Reference") (OtherBodyIndex :type Integer) (bFromSweep :type Boolean) (SweepResult :type "HitResult Structure (by ref)"))
  (bind _launchforwardvelocity (`self.LaunchForwardVelocity`))
  (bind (_returnvalue_x _returnvalue_y) (`KismetMathLibrary.BreakVector` (`KismetMathLibrary.GetForwardVector` (`SceneComponent.K2_GetComponentRotation` (`self.GlidePlatform`)))))
  ;[1 1 1] launch
  (`GameplayStatics.PlaySoundAtLocation` "/Game/Custom/Assets/Audio/platforms/boing.boing" (`self.K2_GetActorLocation` OtherActor) (struct) 1.0 1.0 0.0 null null null null)
  (bind _asnormal_alice (cast `/Game/ThirdPerson/Blueprints/Normal_Alice` OtherActor))
  (`Character.LaunchCharacter` _asnormal_alice (`KismetMathLibrary.MakeVector` (* _returnvalue_x _launchforwardvelocity) (* _returnvalue_y _launchforwardvelocity) (`self.LaunchVelocityZ`)) (`self.XYOverride`) true))

(fn `UserConstructionScript`)